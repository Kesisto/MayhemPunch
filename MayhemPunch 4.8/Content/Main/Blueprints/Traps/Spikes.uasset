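; Spikes is the raised state of a spike trap that kills bots and the player on hit.
; A hit destroys a Bot outright, while a FirstPersonCharacter has its Health set to zero.
; Four seconds after BeginPlay it spawns Spikes_down at its location and destroys itself, switching states by replacing the actor.
; The replacement's transform is built from location alone, so rotation and scale are not passed on.
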(event Collision|EventHit
  (params (MyComp :type Primitive%20Component%20Object%20Reference) (Other :type Actor%20Object%20Reference) (OtherComp :type Primitive%20Component%20Object%20Reference) (bSelfMoved :type Boolean) (HitLocation :type Vector :default "0, 0, 0") (HitNormal :type Vector :default "0, 0, 0") (NormalImpulse :type Vector :default "0, 0, 0") (Hit :type Hit%20Result%20Structure%20%28by%20ref%29))
  (bind _asbot (Utilities|Casting|CastToBot Other)
    (:then
      (Actor|DestroyActor _asbot))
    (:CastFailed
      (bind _asfirst_person_character (Utilities|Casting|CastToFirstPersonCharacter Other))
      (Variables|/Game/Main/Blueprints/FirstPersonCharacter.FirstPersonCharacter_C|SetHealth _asfirst_person_character 0.0))))

(event EventBeginPlay
  (Utilities|FlowControl|DoOnce false
    (:Completed
      (Utilities|FlowControl|Delay 4.0)
      (Game|SpawnActorfromClass "/Game/Main/Blueprints/Traps/Spikes_down.Spikes_down_C" (Math|Conversions|ToTransform(Vector) (Transformation|GetActorLocation)) true 0 0)
      (Actor|DestroyActor))))

(fn ConstructionScript)