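; FireTrap is a trap actor that cycles a fire effect and drains the first-person character's health on overlap.
; A looping BeginPlay sequence uses random delays to swap the mesh material as a warning, spawn P_Fire above the actor, destroy it, then switch to a water material.
; Overlap events set TouchFire, and a delay-throttled Tick repeats small Health decrements while it is set, regardless of whether fire is showing.
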(event EventBeginPlay
  (bind _returnvalue (Transformation|GetActorLocation))
  (bind (_x _y _z) (Math|Vector|BreakVector _returnvalue))
  (Utilities|FlowControl|Delay (Math|Random|RandomFloatinRange 1.0 5.0) :!label _label)
  (Rendering|Material|SetMaterial (Variables|Default|GetStaticMesh) 0 "/Game/ExtraStuff/Maps/Assets/10_Mat.10_Mat")
  (Utilities|FlowControl|Delay 3.0)
  (bind _returnvalue_2 (Effects|SpawnEmitteratLocation "/Game/StarterContent/Particles/P_Fire.P_Fire" (Math|Vector|MakeVector _x _y (+ _z 55.0))))
  (Utilities|FlowControl|Delay (Math|Random|RandomFloatinRange 2.0 6.0))
  (Components|DestroyComponent _returnvalue_2)
  (Utilities|FlowControl|Delay 1.0)
  (Rendering|Material|SetMaterial (Variables|Default|GetStaticMesh) 0 "/Game/StarterContent/Textures/T_Water_Mat.T_Water_Mat")
  (goto _label))

(event EventTick
  (params (DeltaSeconds :type Float%20%28single-precision%29))
  (Utilities|FlowControl|Delay 0.2)
  (if (Variables|Default|GetTouchFire)
    (Variables|/Game/Main/Blueprints/FirstPersonCharacter.FirstPersonCharacter_C|SetHealth (stale Collision|EventActorBeginOverlap _asfirst_person_character) (- (Variables|/Game/Main/Blueprints/FirstPersonCharacter.FirstPersonCharacter_C|GetHealth (stale Collision|EventActorBeginOverlap _asfirst_person_character)) 0.01))))

(event Collision|EventActorEndOverlap
  (params (OtherActor :type Actor%20Object%20Reference))
  (Variables|Default|SetTouchFire false))

(event Collision|EventActorBeginOverlap
  (params (OtherActor :type Actor%20Object%20Reference))
  (Variables|Default|SetTouchFire true)
  (bind _asfirst_person_character (Utilities|Casting|CastToFirstPersonCharacter OtherActor))
  (Variables|/Game/Main/Blueprints/FirstPersonCharacter.FirstPersonCharacter_C|SetHealth _asfirst_person_character (- (Variables|/Game/Main/Blueprints/FirstPersonCharacter.FirstPersonCharacter_C|GetHealth _asfirst_person_character) 0.01)))

(fn ConstructionScript)