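; Golf club pickup that the player equips by walking into its static mesh.
; On overlap it enables input, attaches to the FirstPersonCharacter's Weapon1 socket and sets IsWielding on the OmaFPAnimBlueprint anim instance.
; Right mouse detaches the mesh in place and blocks re-equipping through CanEquip for a short delay, without clearing IsWielding.
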(event OnComponentBeginOverlap(StaticMesh)
  (params (OtherActor :type Actor%20Object%20Reference) (OtherComp :type Primitive%20Component%20Object%20Reference) (OtherBodyIndex :type Integer) (bFromSweep :type Boolean) (SweepResult :type Hit%20Result%20Structure%20%28by%20ref%29))
  (if (Variables|Default|Getcan%20equip)
    (Input|EnableInput (Game|GetPlayerController 0))
    (bind _asfirst_person_character (Utilities|Casting|CastToFirstPersonCharacter OtherActor))
    (Class|Actor|AttachRootComponentto (Variables|/Game/Main/Blueprints/Characters/FirstPersonCharacter.FirstPersonCharacter_C|GetPlayer _asfirst_person_character) "Weapon1" "SnapToTarget" true)
    (bind _asoma_fpanim_blueprint (Utilities|Casting|CastToOmaFPAnimBlueprint (Components|SkeletalMesh|GetAnimInstance (Variables|/Game/Main/Blueprints/Characters/FirstPersonCharacter.FirstPersonCharacter_C|GetPlayer _asfirst_person_character))))
    (Variables|/Game/Main/Blueprints/Animation/OmaFPAnimBlueprint.OmaFPAnimBlueprint_C|SetIsWielding _asoma_fpanim_blueprint true)))

(event Input|MouseEvents|RightMouseButton
  (:Pressed
    (Variables|Default|Setcan%20equip false)
    (Class|SceneComponent|DetachfromParent (Variables|Default|GetStaticMesh) true true)
    (Utilities|FlowControl|Delay 2.0)
    (Variables|Default|Setcan%20equip true)))

(fn ConstructionScript)