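; Bot is an enemy that chases the player and knocks them back on contact.
; Every tick it issues a simple move toward the player character through its controller.
; Hitting the first-person character launches the player along the bot's forward vector with added lift.
; Each hit plays a pitch-randomized punch sound, with a rare random chance of a joke sound instead.
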(event Collision|EventHit
  (params (MyComp :type Primitive%20Component%20Object%20Reference) (Other :type Actor%20Object%20Reference) (OtherComp :type Primitive%20Component%20Object%20Reference) (bSelfMoved :type Boolean) (HitLocation :type Vector :default "0, 0, 0") (HitNormal :type Vector :default "0, 0, 0") (NormalImpulse :type Vector :default "0, 0, 0") (Hit :type Hit%20Result%20Structure%20%28by%20ref%29))
  (bind _returnvalue (Math|Random|RandomFloatinRange 0.6 1.5))
  (bind _returnvalue_2 (Transformation|GetActorForwardVector))
  (bind (_x _y _z) (Math|Vector|BreakVector _returnvalue_2))
  ;[1 1 1] Knockback
  (Utilities|Casting|CastToFirstPersonCharacter Other)
  (Variables|Default|SetIsHit true)
  (if (Variables|Default|GetIsHit)
    (Character|LaunchCharacter (Game|GetPlayerCharacter 0) (* (Math|Vector|MakeVector _x _y (+ _z 0.4)) 1.5e+03) true true)
    (switch int (Math|Random|RandomInteger 101)
      (:Default
        (Audio|PlaySoundatLocation "/Game/Main/Audio/StrongPunch.StrongPunch" "0, 0, 0" 0.3 _returnvalue))
      (:100
        (Audio|PlaySoundatLocation "/Game/Main/Animations/PINGAS.PINGAS" "0, 0, 0" 0.8 _returnvalue)))))

(event EventTick
  (params (DeltaSeconds :type Float%20%28single-precision%29))
  ;[1 1 1] Bot movement
  (AI|Navigation|SimpleMovetoActor (Pawn|GetController) (Game|GetPlayerCharacter 0)))

(fn ConstructionScript)