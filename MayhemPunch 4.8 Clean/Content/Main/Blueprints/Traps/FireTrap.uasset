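; Fire trap actor that periodically bursts flame and drains the first-person character's Health on overlap.
; A BeginPlay loop plays the trap animation, spawns a fire emitter and sound above the actor, destroys the emitter, then repeats after a random pause.
; Overlap sets a touch flag, and a delay-throttled Tick repeats the small damage step until overlap ends.
; Damage does not check whether the flame is active.
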(event EventBeginPlay
  (bind _returnvalue (Transformation|GetActorLocation))
  (bind (_x _y _z) (Math|Vector|BreakVector _returnvalue))
  (bind _returnvalue_2 (+ _z 55.0))
  (bind _returnvalue_3 (Math|Vector|MakeVector _x _y _returnvalue_2))
  (Components|Animation|PlayAnimation (Variables|Default|Gettuliansa_02) "/Game/Main/Blueprints/Traps/tuliansa_03_Anim.tuliansa_03_Anim" false :!label _label)
  (Utilities|FlowControl|Delay 0.25)
  (bind _returnvalue_4 (Effects|SpawnEmitteratLocation "/Game/StarterContent/Particles/Ansatuli.Ansatuli" _returnvalue_3))
  (Audio|PlaySoundatLocation "/Game/Main/Audio/Tulipallo.Tulipallo" _returnvalue_3 0.6 1.0 0.0 "/Game/Main/Audio/TuliansaAttenuation.TuliansaAttenuation")
  (Utilities|FlowControl|Delay 2.5)
  (Components|DestroyComponent _returnvalue_4)
  (Utilities|FlowControl|Delay (Math|Random|RandomFloatinRange 1.0 5.0))
  (goto _label))

(event EventTick
  (params (DeltaSeconds :type Float%20%28single-precision%29))
  ;[1 1 1] damage
  (Utilities|FlowControl|Delay 0.2)
  (if (Variables|Default|GetTouchFire)
    (Variables|/Game/Main/Blueprints/FirstPersonCharacter.FirstPersonCharacter_C|SetHealth (stale Collision|EventActorBeginOverlap _asfirst_person_character) (- (Variables|/Game/Main/Blueprints/FirstPersonCharacter.FirstPersonCharacter_C|GetHealth (stale Collision|EventActorBeginOverlap _asfirst_person_character)) 0.01))))

(event Collision|EventActorEndOverlap
  (params (OtherActor :type Actor%20Object%20Reference))
  ;[1 1 1] damage
  (Variables|Default|SetTouchFire false))

(event Collision|EventActorBeginOverlap
  (params (OtherActor :type Actor%20Object%20Reference))
  ;[1 1 1] damage
  (Variables|Default|SetTouchFire true)
  (bind _asfirst_person_character (Utilities|Casting|CastToFirstPersonCharacter OtherActor))
  (Variables|/Game/Main/Blueprints/FirstPersonCharacter.FirstPersonCharacter_C|SetHealth _asfirst_person_character (- (Variables|/Game/Main/Blueprints/FirstPersonCharacter.FirstPersonCharacter_C|GetHealth _asfirst_person_character) 0.01)))

(fn ConstructionScript)