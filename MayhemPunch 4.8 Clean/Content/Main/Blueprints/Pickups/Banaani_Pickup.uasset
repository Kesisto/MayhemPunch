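; Banana pickup that the first-person character can carry and throw.
; On mesh overlap while equippable, it enables player input, stops physics, snaps to the character's Weapon1 socket and sets IsWielding on the anim Blueprint.
; Right mouse restores physics, detaches it and launches it along the capsule's forward vector, blocking re-equip for a short delay.
; The throw leaves IsWielding and the actor's input enabled.
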(event OnComponentBeginOverlap(Bananamesh)
  (params (OtherActor :type Actor%20Object%20Reference) (OtherComp :type Primitive%20Component%20Object%20Reference) (OtherBodyIndex :type Integer) (bFromSweep :type Boolean) (SweepResult :type Hit%20Result%20Structure%20%28by%20ref%29))
  (if (Variables|Default|GetCan%20equip)
    (Input|EnableInput (Game|GetPlayerController 0))
    (Physics|SetSimulatePhysics (Variables|Default|GetBananamesh) false)
    (bind _asfirst_person_character (Utilities|Casting|CastToFirstPersonCharacter OtherActor))
    (Class|Actor|AttachRootComponentto (Variables|/Game/Main/Blueprints/Characters/FirstPersonCharacter.FirstPersonCharacter_C|GetPlayer _asfirst_person_character) "Weapon1" "SnapToTarget" true)
    (bind _asoma_fpanim_blueprint (Utilities|Casting|CastToOmaFPAnimBlueprint (Components|SkeletalMesh|GetAnimInstance (Variables|/Game/Main/Blueprints/Characters/FirstPersonCharacter.FirstPersonCharacter_C|GetPlayer _asfirst_person_character))))
    (Variables|/Game/Main/Blueprints/Animation/OmaFPAnimBlueprint.OmaFPAnimBlueprint_C|SetIsWielding _asoma_fpanim_blueprint true)))

(event Input|MouseEvents|RightMouseButton
  (bind _bananamesh (Variables|Default|GetBananamesh))
  (:Pressed
    (Variables|Default|SetCan%20equip false)
    (Physics|SetSimulatePhysics _bananamesh true)
    (Class|SceneComponent|DetachfromParent _bananamesh true true)
    (Physics|AddImpulse (Variables|Default|GetBananamesh) (* (Math|Vector|GetForwardVector (Variables|/Script/Engine.Character|GetCapsuleComponent (stale OnComponentBeginOverlap(Bananamesh) _asfirst_person_character))) 2.5e+03) "None" false)
    (Utilities|FlowControl|Delay 1.0)
    (Variables|Default|SetCan%20equip true)))

(fn ConstructionScript)