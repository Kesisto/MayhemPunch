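; Dynamite is an explosive actor that detonates on its first hit.
; A hit pushes the other component along the dynamite's velocity and removes the Sphere, then a DoOnce gate fires the RadialForce impulse with an explosion particle and attached sound.
; The actor destroys itself after a short delay.
; An unconnected Delay leading into the detonation chain never runs.
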(event Collision|EventHit
  (params (MyComp :type Primitive%20Component%20Object%20Reference) (Other :type Actor%20Object%20Reference) (OtherComp :type Primitive%20Component%20Object%20Reference) (bSelfMoved :type Boolean) (HitLocation :type Vector :default "0, 0, 0") (HitNormal :type Vector :default "0, 0, 0") (NormalImpulse :type Vector :default "0, 0, 0") (Hit :type Hit%20Result%20Structure%20%28by%20ref%29))
  (bind _radialforce (Variables|Default|GetRadialForce))
  (bind _returnvalue (Transformation|GetWorldLocation _radialforce))
  ;[1 1 1] BOOM BOOM
  (Physics|AddImpulseatLocation OtherComp (* (Transformation|GetVelocity) 1e+02) (Transformation|GetActorLocation) "None")
  (Components|DestroyComponent (Variables|MyProjectile|GetSphere))
  (Utilities|FlowControl|DoOnce false
    (:Completed
      (Class|RadialForceComponent|FireImpulse _radialforce)
      (bind _returnvalue_2 (Effects|SpawnEmitteratLocation "/Game/StarterContent/Particles/P_Explosion.P_Explosion" _returnvalue))
      (Class|GameplayStatics|PlaySoundAttached "/Game/StarterContent/Audio/Explosion02.Explosion02" _returnvalue_2 "None" _returnvalue "KeepRelativeOffset" false 0.5)
      (Utilities|FlowControl|Delay 6.0)
      (Actor|DestroyActor))))

(fn ConstructionScript)