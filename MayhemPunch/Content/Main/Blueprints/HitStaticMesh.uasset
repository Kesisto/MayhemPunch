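; An explosive projectile actor, HitStaticMesh, that detonates on hit.
; On hit it pushes the struck component with an impulse scaled from its velocity and destroys its sphere component.
; Once only, it fires a radial force impulse, plays an attached sound at the master volume from the CPP_Potkustart game instance, then destroys itself.
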(event Collision|EventHit
  (params (MyComp :type Primitive%20Component%20Object%20Reference) (Other :type Actor%20Object%20Reference) (OtherComp :type Primitive%20Component%20Object%20Reference) (bSelfMoved :type Boolean) (HitLocation :type Vector :default "0, 0, 0") (HitNormal :type Vector :default "0, 0, 0") (NormalImpulse :type Vector :default "0, 0, 0") (Hit :type Hit%20Result%20Structure%20%28by%20ref%29))
  ;[1 1 1] BOOM BOOM
  (Physics|AddImpulseatLocation OtherComp (* (Transformation|GetVelocity) 1e+02) (Transformation|GetActorLocation) "None")
  (Components|DestroyComponent (Variables|MyProjectile|GetSphere))
  (Utilities|FlowControl|DoOnce false
    (:Completed
      (Class|RadialForceComponent|FireImpulse (Variables|Default|GetRadialForce))
      (bind _ascpp_potkustart (Utilities|Casting|CastToCPP_Potkustart (Game|GetGameInstance)))
      (Class|GameplayStatics|PlaySoundAttached 0 0 "None" "0, 0, 0" "KeepRelativeOffset" false (Variables|/Script/MayhemPunch.CPPGameInstance|GetMaster _ascpp_potkustart))
      (Actor|DestroyActor))))

(fn ConstructionScript)