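; Spawner actor that places the weapon pickups (bat, golf club, crowbar, gravity hammer), a banana bunch and single bananas, and respawns them when destroyed.
; On BeginPlay, SpawnAll creates each pickup at its stored transform, then Bindings hooks every OnDestroyed.
; Each respawn event waits a shared Delay, spawns a replacement and rebinds it.
; Bananas spawn from a transform array, but respawn handlers are hard-coded for thirteen indices.
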(event Custom|Banana9Respawn
  (Utilities|FlowControl|Delay (Variables|Default|GetDelay))
  (bind _returnvalue (Game|SpawnActorfromClass "/Game/Main/Blueprints/Pickups/Banaani_Pickup.Banaani_Pickup_C" (Utilities|Array|Get(acopy) (Variables|Spawns|GetBananaSpawn) 9) true 0 0))
  (Utilities|Array|SetArrayElem (Variables|Pickups|GetBanana) 9 _returnvalue)
  (CallFunction|Banana9Dead))

(event Custom|Banana9Dead
  (Game|BindEventtoOnDestroyed (Utilities|Array|Get(acopy) (Variables|Pickups|GetBanana) 9) (delegate Custom|Banana9Respawn)))

(event Custom|Banana10Respawn
  (Utilities|FlowControl|Delay (Variables|Default|GetDelay))
  (bind _returnvalue (Game|SpawnActorfromClass "/Game/Main/Blueprints/Pickups/Banaani_Pickup.Banaani_Pickup_C" (Utilities|Array|Get(acopy) (Variables|Spawns|GetBananaSpawn) 10) true 0 0))
  (Utilities|Array|SetArrayElem (Variables|Pickups|GetBanana) 10 _returnvalue)
  (CallFunction|Banana10Dead))

(event Custom|Banana10Dead
  (Game|BindEventtoOnDestroyed (Utilities|Array|Get(acopy) (Variables|Pickups|GetBanana) 10) (delegate Custom|Banana10Respawn)))

(event Custom|Banana6Respawn
  (Utilities|FlowControl|Delay (Variables|Default|GetDelay))
  (bind _returnvalue (Game|SpawnActorfromClass "/Game/Main/Blueprints/Pickups/Banaani_Pickup.Banaani_Pickup_C" (Utilities|Array|Get(acopy) (Variables|Spawns|GetBananaSpawn) 6) true 0 0))
  (Utilities|Array|SetArrayElem (Variables|Pickups|GetBanana) 6 _returnvalue)
  (CallFunction|Banana6Dead))

(event Custom|Banana6Dead
  (Game|BindEventtoOnDestroyed (Utilities|Array|Get(acopy) (Variables|Pickups|GetBanana) 6) (delegate Custom|Banana6Respawn)))

(event Custom|Banana7Respawn
  (Utilities|FlowControl|Delay (Variables|Default|GetDelay))
  (bind _returnvalue (Game|SpawnActorfromClass "/Game/Main/Blueprints/Pickups/Banaani_Pickup.Banaani_Pickup_C" (Utilities|Array|Get(acopy) (Variables|Spawns|GetBananaSpawn) 7) true 0 0))
  (Utilities|Array|SetArrayElem (Variables|Pickups|GetBanana) 7 _returnvalue)
  (CallFunction|Banana7Dead))

(event Custom|Banana7Dead
  (Game|BindEventtoOnDestroyed (Utilities|Array|Get(acopy) (Variables|Pickups|GetBanana) 7) (delegate Custom|Banana7Respawn)))

(event Custom|Banana8Respawn
  (Utilities|FlowControl|Delay (Variables|Default|GetDelay))
  (bind _returnvalue (Game|SpawnActorfromClass "/Game/Main/Blueprints/Pickups/Banaani_Pickup.Banaani_Pickup_C" (Utilities|Array|Get(acopy) (Variables|Spawns|GetBananaSpawn) 8) true 0 0))
  (Utilities|Array|SetArrayElem (Variables|Pickups|GetBanana) 8 _returnvalue)
  (CallFunction|Banana8Dead))

(event Custom|Banana8Dead
  (Game|BindEventtoOnDestroyed (Utilities|Array|Get(acopy) (Variables|Pickups|GetBanana) 8) (delegate Custom|Banana8Respawn)))

(event Custom|Banana0Respawn
  (Utilities|FlowControl|Delay (Variables|Default|GetDelay))
  (bind _returnvalue (Game|SpawnActorfromClass "/Game/Main/Blueprints/Pickups/Banaani_Pickup.Banaani_Pickup_C" (Utilities|Array|Get(acopy) (Variables|Spawns|GetBananaSpawn)) true 0 0))
  (Utilities|Array|SetArrayElem (Variables|Pickups|GetBanana) 0 _returnvalue)
  (CallFunction|Banana0Dead))

(event Custom|Banana0Dead
  (Game|BindEventtoOnDestroyed (Utilities|Array|Get(acopy) (Variables|Pickups|GetBanana)) (delegate Custom|Banana0Respawn)))

(event Custom|Banana1Respawn
  (Utilities|FlowControl|Delay (Variables|Default|GetDelay))
  (bind _returnvalue (Game|SpawnActorfromClass "/Game/Main/Blueprints/Pickups/Banaani_Pickup.Banaani_Pickup_C" (Utilities|Array|Get(acopy) (Variables|Spawns|GetBananaSpawn) 1) true 0 0))
  (Utilities|Array|SetArrayElem (Variables|Pickups|GetBanana) 1 _returnvalue)
  (CallFunction|Banana1Dead))

(event Custom|Banana1Dead
  (Game|BindEventtoOnDestroyed (Utilities|Array|Get(acopy) (Variables|Pickups|GetBanana) 1) (delegate Custom|Banana1Respawn)))

(event Custom|Banana2Respawn
  (Utilities|FlowControl|Delay (Variables|Default|GetDelay))
  (bind _returnvalue (Game|SpawnActorfromClass "/Game/Main/Blueprints/Pickups/Banaani_Pickup.Banaani_Pickup_C" (Utilities|Array|Get(acopy) (Variables|Spawns|GetBananaSpawn) 2) true 0 0))
  (Utilities|Array|SetArrayElem (Variables|Pickups|GetBanana) 2 _returnvalue)
  (CallFunction|Banana2Dead))

(event Custom|Banana2Dead
  (Game|BindEventtoOnDestroyed (Utilities|Array|Get(acopy) (Variables|Pickups|GetBanana) 2) (delegate Custom|Banana2Respawn)))

(event Custom|Banana3Respawn
  (Utilities|FlowControl|Delay (Variables|Default|GetDelay))
  (bind _returnvalue (Game|SpawnActorfromClass "/Game/Main/Blueprints/Pickups/Banaani_Pickup.Banaani_Pickup_C" (Utilities|Array|Get(acopy) (Variables|Spawns|GetBananaSpawn) 3) true 0 0))
  (Utilities|Array|SetArrayElem (Variables|Pickups|GetBanana) 3 _returnvalue)
  (CallFunction|Banana3Dead))

(event Custom|Banana3Dead
  (Game|BindEventtoOnDestroyed (Utilities|Array|Get(acopy) (Variables|Pickups|GetBanana) 3) (delegate Custom|Banana3Respawn)))

(event Custom|Banana4Respawn
  (Utilities|FlowControl|Delay (Variables|Default|GetDelay))
  (bind _returnvalue (Game|SpawnActorfromClass "/Game/Main/Blueprints/Pickups/Banaani_Pickup.Banaani_Pickup_C" (Utilities|Array|Get(acopy) (Variables|Spawns|GetBananaSpawn) 4) true 0 0))
  (Utilities|Array|SetArrayElem (Variables|Pickups|GetBanana) 4 _returnvalue)
  (CallFunction|Banana4Dead))

(event Custom|Banana4Dead
  (Game|BindEventtoOnDestroyed (Utilities|Array|Get(acopy) (Variables|Pickups|GetBanana) 4) (delegate Custom|Banana4Respawn)))

(event Custom|Banana5Respawn
  (Utilities|FlowControl|Delay (Variables|Default|GetDelay))
  (bind _returnvalue (Game|SpawnActorfromClass "/Game/Main/Blueprints/Pickups/Banaani_Pickup.Banaani_Pickup_C" (Utilities|Array|Get(acopy) (Variables|Spawns|GetBananaSpawn) 5) true 0 0))
  (Utilities|Array|SetArrayElem (Variables|Pickups|GetBanana) 5 _returnvalue)
  (CallFunction|Banana5Dead))

(event Custom|Banana5Dead
  (Game|BindEventtoOnDestroyed (Utilities|Array|Get(acopy) (Variables|Pickups|GetBanana) 5) (delegate Custom|Banana5Respawn)))

(event Custom|Banana11Respawn
  (Utilities|FlowControl|Delay (Variables|Default|GetDelay))
  (bind _returnvalue (Game|SpawnActorfromClass "/Game/Main/Blueprints/Pickups/Banaani_Pickup.Banaani_Pickup_C" (Utilities|Array|Get(acopy) (Variables|Spawns|GetBananaSpawn) 11) true 0 0))
  (Utilities|Array|SetArrayElem (Variables|Pickups|GetBanana) 11 _returnvalue)
  (CallFunction|Banana11Dead))

(event Custom|Banana11Dead
  (Game|BindEventtoOnDestroyed (Utilities|Array|Get(acopy) (Variables|Pickups|GetBanana) 11) (delegate Custom|Banana11Respawn)))

(event Custom|BaseballRespawn
  (Utilities|FlowControl|Delay (Variables|Default|GetDelay))
  (bind _returnvalue (Game|SpawnActorfromClass "/Game/Main/Blueprints/Pickups/BaseballBat_Pickup.BaseballBat_Pickup_C" (Variables|Spawns|GetBaseballBatSpawn) true 0 0))
  (Variables|Pickups|SetBaseballBat _returnvalue)
  (CallFunction|BaseballBatDead))

(event Custom|Bindings
  (bind _banana (Variables|Pickups|GetBanana))
  (Game|BindEventtoOnDestroyed (Variables|Pickups|GetBaseballBat) (delegate Custom|BaseballRespawn))
  (Game|BindEventtoOnDestroyed (Variables|Pickups|GetGolfClub) (delegate Custom|GolfClubRespawn))
  (Game|BindEventtoOnDestroyed (Variables|Pickups|GetCrowbar) (delegate Custom|CrowbarRespawn))
  (Game|BindEventtoOnDestroyed (Variables|Pickups|GetGravityHammer) (delegate Custom|GravityHammerRespawn))
  (Game|BindEventtoOnDestroyed (Variables|Pickups|GetBananas) (delegate Custom|BananasRespawn))
  (Game|BindEventtoOnDestroyed (Utilities|Array|Get(acopy) _banana) (delegate Custom|Banana0Respawn))
  (Game|BindEventtoOnDestroyed (Utilities|Array|Get(acopy) _banana 1) (delegate Custom|Banana1Respawn))
  (Game|BindEventtoOnDestroyed (Utilities|Array|Get(acopy) _banana 2) (delegate Custom|Banana2Respawn))
  (Game|BindEventtoOnDestroyed (Utilities|Array|Get(acopy) _banana 3) (delegate Custom|Banana3Respawn))
  (Game|BindEventtoOnDestroyed (Utilities|Array|Get(acopy) _banana 4) (delegate Custom|Banana4Respawn))
  (Game|BindEventtoOnDestroyed (Utilities|Array|Get(acopy) _banana 5) (delegate Custom|Banana5Respawn))
  (Game|BindEventtoOnDestroyed (Utilities|Array|Get(acopy) _banana 6) (delegate Custom|Banana6Respawn))
  (Game|BindEventtoOnDestroyed (Utilities|Array|Get(acopy) _banana 7) (delegate Custom|Banana7Respawn))
  (Game|BindEventtoOnDestroyed (Utilities|Array|Get(acopy) _banana 8) (delegate Custom|Banana8Respawn))
  (Game|BindEventtoOnDestroyed (Utilities|Array|Get(acopy) _banana 9) (delegate Custom|Banana9Respawn))
  (Game|BindEventtoOnDestroyed (Utilities|Array|Get(acopy) _banana 10) (delegate Custom|Banana10Respawn))
  (Game|BindEventtoOnDestroyed (Utilities|Array|Get(acopy) _banana 11) (delegate Custom|Banana11Respawn))
  (Game|BindEventtoOnDestroyed (Utilities|Array|Get(acopy) _banana 12) (delegate Custom|Banana12Respawn)))

(event Custom|BananasRespawn
  (Utilities|FlowControl|Delay (Variables|Default|GetDelay))
  (bind _returnvalue (Game|SpawnActorfromClass "/Game/Main/Blueprints/Pickups/BanaaniTerttu.BanaaniTerttu_C" (Variables|Spawns|GetBananasSpawn) true 0 0))
  (Variables|Pickups|SetBananas _returnvalue)
  (CallFunction|BananasDead))

(event Custom|GolfClubRespawn
  (Utilities|FlowControl|Delay (Variables|Default|GetDelay))
  (bind _returnvalue (Game|SpawnActorfromClass "/Game/Main/Blueprints/Pickups/GolfClub_Pickup.GolfClub_Pickup_C" (Variables|Spawns|GetGolfClubSpawn) true 0 0))
  (Variables|Pickups|SetGolfClub _returnvalue)
  (CallFunction|GolfClubDead))

(event Custom|CrowbarRespawn
  (Utilities|FlowControl|Delay (Variables|Default|GetDelay))
  (bind _returnvalue (Game|SpawnActorfromClass "/Game/Main/Blueprints/Pickups/Sorkkarauta_Pickup.Sorkkarauta_Pickup_C" (Variables|Spawns|GetCrowbarSpawn) true 0 0))
  (Variables|Pickups|SetCrowbar _returnvalue)
  (CallFunction|CrowbarDead))

(event Custom|GravityHammerRespawn
  (Utilities|FlowControl|Delay (Variables|Default|GetDelay))
  (bind _returnvalue (Game|SpawnActorfromClass "/Game/Main/Blueprints/Pickups/GravHam_Pickup.GravHam_Pickup_C" (Variables|Spawns|GetGravityHammerSpawn) true 0 0))
  (Variables|Pickups|SetGravityHammer _returnvalue)
  (CallFunction|GravityHammerDead))

(event Custom|Banana12Respawn
  (Utilities|FlowControl|Delay (Variables|Default|GetDelay))
  (bind _returnvalue (Game|SpawnActorfromClass "/Game/Main/Blueprints/Pickups/Banaani_Pickup.Banaani_Pickup_C" (Utilities|Array|Get(acopy) (Variables|Spawns|GetBananaSpawn) 12) true 0 0))
  (Utilities|Array|SetArrayElem (Variables|Pickups|GetBanana) 12 _returnvalue)
  (CallFunction|Banana12Dead))

(event Custom|BaseballBatDead
  (Game|BindEventtoOnDestroyed (Variables|Pickups|GetBaseballBat) (delegate Custom|BaseballRespawn)))

(event Custom|GolfClubDead
  (Game|BindEventtoOnDestroyed (Variables|Pickups|GetGolfClub) (delegate Custom|GolfClubRespawn)))

(event Custom|CrowbarDead
  (Game|BindEventtoOnDestroyed (Variables|Pickups|GetCrowbar) (delegate Custom|CrowbarRespawn)))

(event Custom|GravityHammerDead
  (Game|BindEventtoOnDestroyed (Variables|Pickups|GetGravityHammer) (delegate Custom|GravityHammerRespawn)))

(event Custom|BananasDead
  (Game|BindEventtoOnDestroyed (Variables|Pickups|GetBananas) (delegate Custom|BananasRespawn)))

(event Custom|Banana12Dead
  (Game|BindEventtoOnDestroyed (Utilities|Array|Get(acopy) (Variables|Pickups|GetBanana) 12) (delegate Custom|Banana12Respawn)))

(event EventBeginPlay
  (CallFunction|SpawnAll)
  (CallFunction|Bindings))

(fn ConstructionScript)

(fn SpawnAll
  (bind _returnvalue (Game|SpawnActorfromClass "/Game/Main/Blueprints/Pickups/BaseballBat_Pickup.BaseballBat_Pickup_C" (Variables|Spawns|GetBaseballBatSpawn) false 0 0))
  (Variables|Pickups|SetBaseballBat _returnvalue)
  (bind _returnvalue_2 (Game|SpawnActorfromClass "/Game/Main/Blueprints/Pickups/GolfClub_Pickup.GolfClub_Pickup_C" (Variables|Spawns|GetGolfClubSpawn) false 0 0))
  (Variables|Pickups|SetGolfClub _returnvalue_2)
  (bind _returnvalue_3 (Game|SpawnActorfromClass "/Game/Main/Blueprints/Pickups/Sorkkarauta_Pickup.Sorkkarauta_Pickup_C" (Variables|Spawns|GetCrowbarSpawn) false 0 0))
  (Variables|Pickups|SetCrowbar _returnvalue_3)
  (bind _returnvalue_4 (Game|SpawnActorfromClass "/Game/Main/Blueprints/Pickups/GravHam_Pickup.GravHam_Pickup_C" (Variables|Spawns|GetGravityHammerSpawn) false 0 0))
  (Variables|Pickups|SetGravityHammer _returnvalue_4)
  (bind _returnvalue_5 (Game|SpawnActorfromClass "/Game/Main/Blueprints/Pickups/BanaaniTerttu.BanaaniTerttu_C" (Variables|Spawns|GetBananasSpawn) false 0 0))
  (Variables|Pickups|SetBananas _returnvalue_5)
  (for _array_element (Variables|Spawns|GetBananaSpawn)
    (bind _returnvalue_6 (Game|SpawnActorfromClass "/Game/Main/Blueprints/Pickups/Banaani_Pickup.Banaani_Pickup_C" _array_element false 0 0))
    (Utilities|Array|Add (Variables|Pickups|GetBanana) _returnvalue_6)))