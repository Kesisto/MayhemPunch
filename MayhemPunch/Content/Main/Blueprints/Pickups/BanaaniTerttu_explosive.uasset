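; Explosive banana bunch projectile that bursts into a cluster of smaller explosive bananas after bouncing.
; A bounce counter lets two bounces pass, then a short delay precedes a radial impulse, blast sound, explosion emitter and self-destruction.
; A DoOnce after the destroy call spawns twelve Banaani_Explosive actors in place and sets their FirstBanana flags.
; The velocity calls between spawns target this actor's own ProjectileMovement, not the spawned bananas'.
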(event OnProjectileBounce(ProjectileMovement)
  (params (ImpactResult :type Hit%20Result%20Structure%20%28by%20ref%29) (ImpactVelocity :type Vector%20%28by%20ref%29 :default "0, 0, 0"))
  (bind _staticmesh (Variables|Default|GetStaticMesh))
  (bind _returnvalue (Transformation|GetWorldLocation _staticmesh))
  (bind _returnvalue_2 (Math|Conversions|ToTransform(Vector) _returnvalue))
  (bind _returnvalue_3 (Math|Conversions|ToTransform(Vector) _returnvalue))
  (bind (_x _y _z) (Math|Vector|BreakVector _returnvalue))
  (if (>= (Variables|Default|GetBounceCounter) 2)
    (Utilities|FlowControl|Delay 0.3)
    (Class|RadialForceComponent|FireImpulse (Variables|Default|GetRadialForce))
    (Class|GameplayStatics|PlaySoundAttached "/Game/Main/Audio/Enviroment/Banana_Blast.Banana_Blast" _staticmesh "None" _returnvalue "KeepRelativeOffset" false 1.0 1.0 0.0 "/Game/Main/Audio/Ansa_Attenuation.Ansa_Attenuation")
    (Effects|SpawnEmitteratLocation "/Game/Main/Visuals/Particles/Banana_Explosion.Banana_Explosion" (Math|Vector|MakeVector _x _y (+ _z 5e+01)))
    (Actor|DestroyActor)
    (Utilities|FlowControl|DoOnce false
      (:Completed
        (bind _returnvalue_4 (Game|SpawnActorfromClass "/Game/Main/Blueprints/Pickups/Banaani_Explosive.Banaani_Explosive_C" _returnvalue_3 true 0 0))
        (Game|Components|ProjectileMovement|SetVelocityinLocalSpace (Variables|Default|GetProjectileMovement) "0.500000,0.000000,1.000000")
        (Variables|/Game/Main/Blueprints/Pickups/Banaani_Explosive.Banaani_Explosive_C|SetFirstBanana _returnvalue_4 false)
        (bind _returnvalue_5 (Game|SpawnActorfromClass "/Game/Main/Blueprints/Pickups/Banaani_Explosive.Banaani_Explosive_C" _returnvalue_3 true 0 0))
        (Game|Components|ProjectileMovement|SetVelocityinLocalSpace (Variables|Default|GetProjectileMovement) "-0.500000,-0.500000,1.000000")
        (Variables|/Game/Main/Blueprints/Pickups/Banaani_Explosive.Banaani_Explosive_C|SetFirstBanana _returnvalue_5 true)
        (bind _returnvalue_6 (Game|SpawnActorfromClass "/Game/Main/Blueprints/Pickups/Banaani_Explosive.Banaani_Explosive_C" _returnvalue_3 true 0 0))
        (Game|Components|ProjectileMovement|SetVelocityinLocalSpace (Variables|Default|GetProjectileMovement) "-0.500000,-0.500000,1.000000")
        (Variables|/Game/Main/Blueprints/Pickups/Banaani_Explosive.Banaani_Explosive_C|SetFirstBanana _returnvalue_6 true)
        (bind _returnvalue_7 (Game|SpawnActorfromClass "/Game/Main/Blueprints/Pickups/Banaani_Explosive.Banaani_Explosive_C" _returnvalue_3 true 0 0))
        (Game|Components|ProjectileMovement|SetVelocityinLocalSpace (Variables|Default|GetProjectileMovement) "0.000000,0.500000,1.000000")
        (Variables|/Game/Main/Blueprints/Pickups/Banaani_Explosive.Banaani_Explosive_C|SetFirstBanana _returnvalue_7 true)
        (bind _returnvalue_8 (Game|SpawnActorfromClass "/Game/Main/Blueprints/Pickups/Banaani_Explosive.Banaani_Explosive_C" _returnvalue_3 true 0 0))
        (Game|Components|ProjectileMovement|SetVelocityinLocalSpace (Variables|Default|GetProjectileMovement) "0.000000,0.500000,1.000000")
        (Variables|/Game/Main/Blueprints/Pickups/Banaani_Explosive.Banaani_Explosive_C|SetFirstBanana _returnvalue_8 true)
        (bind _returnvalue_9 (Game|SpawnActorfromClass "/Game/Main/Blueprints/Pickups/Banaani_Explosive.Banaani_Explosive_C" _returnvalue_3 true 0 0))
        (Game|Components|ProjectileMovement|SetVelocityinLocalSpace (Variables|Default|GetProjectileMovement) "0.000000,0.500000,1.000000")
        (Variables|/Game/Main/Blueprints/Pickups/Banaani_Explosive.Banaani_Explosive_C|SetFirstBanana _returnvalue_9 true)
        (bind _returnvalue_10 (Game|SpawnActorfromClass "/Game/Main/Blueprints/Pickups/Banaani_Explosive.Banaani_Explosive_C" _returnvalue_2 true 0 0))
        (Game|Components|ProjectileMovement|SetVelocityinLocalSpace (Variables|Default|GetProjectileMovement) "0.500000,0.000000,1.000000")
        (Variables|/Game/Main/Blueprints/Pickups/Banaani_Explosive.Banaani_Explosive_C|SetFirstBanana _returnvalue_10 false)
        (bind _returnvalue_11 (Game|SpawnActorfromClass "/Game/Main/Blueprints/Pickups/Banaani_Explosive.Banaani_Explosive_C" _returnvalue_2 true 0 0))
        (Game|Components|ProjectileMovement|SetVelocityinLocalSpace (Variables|Default|GetProjectileMovement) "-0.500000,-0.500000,1.000000")
        (Variables|/Game/Main/Blueprints/Pickups/Banaani_Explosive.Banaani_Explosive_C|SetFirstBanana _returnvalue_11 true)
        (bind _returnvalue_12 (Game|SpawnActorfromClass "/Game/Main/Blueprints/Pickups/Banaani_Explosive.Banaani_Explosive_C" _returnvalue_2 true 0 0))
        (Game|Components|ProjectileMovement|SetVelocityinLocalSpace (Variables|Default|GetProjectileMovement) "-0.500000,-0.500000,1.000000")
        (Variables|/Game/Main/Blueprints/Pickups/Banaani_Explosive.Banaani_Explosive_C|SetFirstBanana _returnvalue_12 true)
        (bind _returnvalue_13 (Game|SpawnActorfromClass "/Game/Main/Blueprints/Pickups/Banaani_Explosive.Banaani_Explosive_C" _returnvalue_2 true 0 0))
        (Game|Components|ProjectileMovement|SetVelocityinLocalSpace (Variables|Default|GetProjectileMovement) "0.000000,0.500000,1.000000")
        (Variables|/Game/Main/Blueprints/Pickups/Banaani_Explosive.Banaani_Explosive_C|SetFirstBanana _returnvalue_13 true)
        (bind _returnvalue_14 (Game|SpawnActorfromClass "/Game/Main/Blueprints/Pickups/Banaani_Explosive.Banaani_Explosive_C" _returnvalue_2 true 0 0))
        (Game|Components|ProjectileMovement|SetVelocityinLocalSpace (Variables|Default|GetProjectileMovement) "0.000000,0.500000,1.000000")
        (Variables|/Game/Main/Blueprints/Pickups/Banaani_Explosive.Banaani_Explosive_C|SetFirstBanana _returnvalue_14 true)
        (bind _returnvalue_15 (Game|SpawnActorfromClass "/Game/Main/Blueprints/Pickups/Banaani_Explosive.Banaani_Explosive_C" _returnvalue_2 true 0 0))
        (Game|Components|ProjectileMovement|SetVelocityinLocalSpace (Variables|Default|GetProjectileMovement) "0.000000,0.500000,1.000000")
        (Variables|/Game/Main/Blueprints/Pickups/Banaani_Explosive.Banaani_Explosive_C|SetFirstBanana _returnvalue_15 true)))
    (else
      (Variables|Default|SetBounceCounter (+ (Variables|Default|GetBounceCounter) 1)))))

(fn ConstructionScript)