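; BanaaniTerttu is a banana pickup that spins in the world until the player collects it.
; On capsule overlap with a FirstPersonCharacter, it increments that character's BananaCount, writes CanEquip into slot 4 of EquipableWeapons, then destroys itself.
; Tick applies a yaw rotation scaled by delta time and YawPerSec for a frame-rate-independent spin.
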(event OnComponentBeginOverlap(Capsule)
  (params (OtherActor :type Actor%20Object%20Reference) (OtherComp :type Primitive%20Component%20Object%20Reference) (OtherBodyIndex :type Integer) (bFromSweep :type Boolean) (SweepResult :type Hit%20Result%20Structure%20%28by%20ref%29))
  (bind _asfirst_person_character (Utilities|Casting|CastToFirstPersonCharacter OtherActor))
  (Variables|/Game/Main/Blueprints/Characters/FirstPersonCharacter.FirstPersonCharacter_C|SetBananaCount _asfirst_person_character (+ (Variables|/Game/Main/Blueprints/Characters/FirstPersonCharacter.FirstPersonCharacter_C|GetBananaCount _asfirst_person_character) 1))
  (Utilities|Array|SetArrayElem (Variables|/Game/Main/Blueprints/Characters/FirstPersonCharacter.FirstPersonCharacter_C|GetEquipableWeapons _asfirst_person_character) 4 (Variables|Default|GetCan%20equip))
  (Actor|DestroyActor))

(event EventTick
  (params (DeltaSeconds :type Float%20%28single-precision%29))
  (Transformation|AddActorLocalRotation (Class|KismetMathLibrary|MakeRot 0.0 (* DeltaSeconds (Variables|Default|GetYawPerSec)) 0.0) false))

(fn ConstructionScript)