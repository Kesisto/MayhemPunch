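; Explosive banana projectile that bounces, then blows up with a radial impulse, sound and explosion effect.
; A bounce counter triggers the blast, after a short delay, on the bounce that follows two counted ones.
; If FirstBanana is set, it spawns four more copies at its location after calling DestroyActor.
; The velocity call after each spawn targets this actor's own ProjectileMovement, not the new banana's.
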(event OnProjectileBounce(ProjectileMovement)
  (params (ImpactResult :type Hit%20Result%20Structure%20%28by%20ref%29) (ImpactVelocity :type Vector%20%28by%20ref%29 :default "0, 0, 0"))
  (bind _staticmesh (Variables|Default|GetStaticMesh))
  (bind _returnvalue (Transformation|GetWorldLocation _staticmesh))
  (bind _returnvalue_2 (Math|Conversions|ToTransform(Vector) _returnvalue))
  (bind (_x _y _z) (Math|Vector|BreakVector _returnvalue))
  (if (>= (Variables|Default|GetBounceCounter) 2)
    (Utilities|FlowControl|Delay 0.3)
    (Class|RadialForceComponent|FireImpulse (Variables|Default|GetRadialForce))
    (Class|GameplayStatics|PlaySoundAttached "/Game/Main/Audio/Enviroment/Banana_Blast.Banana_Blast" _staticmesh "None" _returnvalue "KeepRelativeOffset" false 1.0 1.0 0.0 "/Game/Main/Audio/Ansa_Attenuation.Ansa_Attenuation")
    (Effects|SpawnEmitteratLocation "/Game/Main/Visuals/Particles/Banana_Explosion.Banana_Explosion" (Math|Vector|MakeVector _x _y (+ _z 5e+01)))
    (Actor|DestroyActor)
    (if (Variables|Default|GetFirstBanana)
      (Game|SpawnActorfromClass "Banaani_Explosive_C" _returnvalue_2 true 0 0)
      (Game|Components|ProjectileMovement|SetVelocityinLocalSpace (Variables|Default|GetProjectileMovement) "0.500000,0.000000,1.000000")
      (Game|SpawnActorfromClass "Banaani_Explosive_C" _returnvalue_2 true 0 0)
      (Game|Components|ProjectileMovement|SetVelocityinLocalSpace (Variables|Default|GetProjectileMovement) "-0.500000,-0.500000,1.000000")
      (Game|SpawnActorfromClass "Banaani_Explosive_C" _returnvalue_2 true 0 0)
      (Game|Components|ProjectileMovement|SetVelocityinLocalSpace (Variables|Default|GetProjectileMovement) "-0.500000,-0.500000,1.000000")
      (Game|SpawnActorfromClass "Banaani_Explosive_C" _returnvalue_2 true 0 0)
      (Game|Components|ProjectileMovement|SetVelocityinLocalSpace (Variables|Default|GetProjectileMovement) "0.000000,0.500000,1.000000"))
    (else
      (Variables|Default|SetBounceCounter (+ (Variables|Default|GetBounceCounter) 1)))))

(fn ConstructionScript)