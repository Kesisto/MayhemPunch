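; Game instance that manages the game's UI flow and session hosting through a state machine covering startup, loading, main menu, How to Play, error and play.
; TransitionState ignores same-state requests and cleans up the outgoing state, removing its widget or destroying the session when leaving Play.
; Screen events lazily create, cache and show widgets with UI-only input.
; HostGame creates a session and opens Level1 as a listen server, or shows an error dialog on failure.
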(event Custom|DestroySessionCaller
  ;[1 1 1] Destroy it, it must be taken deep into Mordor and cast back into the fiery chasm from whence it came
  (|DestroySession (Game|GetPlayerController 0)))

(event Custom|Show%20Loading%20Screen
  (bind _returnvalue (Game|GetPlayerController 0))
  ;[1 1 1] Show Loading Screen
  (Utilities|TransitionState "NewEnumerator1"
    (:NewState
      (Utilities|IsValid (Variables|Widgets|GetLoadingScreenWidget)
        (:Is%20Valid
          _)
        (:Is%20Not%20Valid
          (bind _returnvalue_2 (UserInterface|CreateWidget "/Game/Main/Blueprints/Widgets/LoadingScreen.LoadingScreen_C" _returnvalue))
          (bind _output_get (Variables|Widgets|SetLoadingScreenWidget _returnvalue_2))))
      (UserInterface|Viewport|AddtoViewport _output_get 0)
      (Input|SetInputModeUIOnly _returnvalue (Variables|Widgets|GetLoadingScreenWidget) false))))

(event Custom|Host%20Game
  ;[1 1 1] Host Game - Called from main menu
  (CallFunction|ShowLoadingScreen)
  (|Session (Game|GetPlayerController 0) (Variables|Misc|GetMaxNumberOfPlayers) (Variables|Misc|GetEnableLAN)
    (:OnSuccess
      (Game|OpenLevel(byName) (Variables|Levels|GetLevel1) true "listen")
      (Utilities|TransitionState "NewEnumerator5"))
    (:OnFailure
      (Utilities|Error "Failed to create session"))))

(event Custom|Show%20Main%20Menu
  (bind _returnvalue (Game|GetPlayerController 0))
  ;[1 1 1] Show Main menu Event
  (Utilities|CurrentState "NewEnumerator5"
    (:True
      (Game|OpenLevel(byName) (Variables|Levels|GetLevelMainMenu)))
    (:False
      _))
  (Utilities|TransitionState "NewEnumerator2"
    (:NewState
      (Utilities|IsValid (Variables|Widgets|GetMainMenuWidget)
        (:Is%20Valid
          _)
        (:Is%20Not%20Valid
          (bind _returnvalue_2 (UserInterface|CreateWidget "/Game/Main/Blueprints/Widgets/MainMenu.MainMenu_C" _returnvalue))
          (Variables|Widgets|SetMainMenuWidget _returnvalue_2)))
      (Input|SetInputModeUIOnly _returnvalue (Variables|Widgets|GetMainMenuWidget) false)
      (UserInterface|Viewport|AddtoViewport (Variables|Widgets|GetMainMenuWidget) 0))))

(event Custom|Show%20HtP
  (bind _returnvalue (Game|GetPlayerController 0))
  ;[1 1 1] How To Play
  (Utilities|TransitionState "NewEnumerator4"
    (:NewState
      (Utilities|IsValid (Variables|Widgets|GetOptionsWidget)
        (:Is%20Valid
          _)
        (:Is%20Not%20Valid
          (bind _returnvalue_2 (UserInterface|CreateWidget "/Game/Main/Blueprints/Widgets/HowToPlay.HowToPlay_C" _returnvalue))
          (bind _output_get (Variables|Widgets|SetOptionsWidget _returnvalue_2))))
      (UserInterface|Viewport|AddtoViewport _output_get 0)
      (Input|SetInputModeUIOnly _returnvalue _output_get false))))

(fn BeginPlayandShowMainMenu
  (CallFunction|ShowLoadingScreen)
  (CallFunction|ShowMainMenu))

(fn HideWidget
  (params (Widget :type Widget%20Object%20Reference))
  (Widget|RemovefromParent Widget))

(fn StartPlaying
  (Utilities|TransitionState "NewEnumerator5"
    (:NewState
      (Input|SetInputModeGameOnly (Game|GetPlayerController 0)))))