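; Bot AI controller that starts a bot's behavior and physics setup when it possesses a pawn.
; On possess it runs the BotTree behavior tree and resets the blackboard's Route key to zero.
; It also enables physics simulation on skeletal mesh bodies below a named bone, with blend weight set to zero so the simulation starts with no visible influence.
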(event EventOnPossess
  (params (PossessedPawn :type Pawn%20Object%20Reference))
  (bind _bonename (Variables|Default|GetBoneName))
  ;[1 1 1] Initialize Bot AI
  (AI|RunBehaviorTree "/Game/Main/Blueprints/Behavior/botTree.botTree")
  (Class|BlackboardComponent|SetValueasInt (AI|GetBlackboard PossessedPawn) (Utilities|Name|MakeLiteralName "Route"))
  (Variables|Default|SetBlendWeight 0.0)
  (Class|SkeletalMeshComponent|SetAllBodiesBelowSimulatePhysics (Variables|Default|GetSkeletalMesh) _bonename true)
  (Class|SkeletalMeshComponent|SetAllBodiesBelowPhysicsBlendWeight (Variables|Default|GetSkeletalMesh) _bonename (Variables|Default|GetBlendWeight) false))

(fn ConstructionScript)