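; Fire trap that periodically shoots flames and burns player characters and bots inside its box.
; A looping BeginPlay chain toggles LuukkuAuki (hatch open), spawning a flame emitter and volume-scaled sound, then closing after a fixed burn and waiting a random interval.
; While open, Tick polls box overlaps and calls FeuerFrei on each character, tagging bot damage with its dealer.
; Bots leaving overlap get their DeathBy cause changed after a short delay.
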(event EventBeginPlay
  (bind _returnvalue (Transformation|GetActorLocation))
  (bind (_x _y _z) (Math|Vector|BreakVector _returnvalue))
  (bind _returnvalue_2 (+ _z 55.0))
  (bind _returnvalue_3 (Math|Vector|MakeVector _x _y _returnvalue_2))
  ;[1 1 1] Luukun aukeaminen
  (Utilities|FlowControl|Delay 0.25 :!label _label)
  (Variables|Default|SetLuukkuAuki true)
  (bind _returnvalue_4 (Effects|SpawnEmitteratLocation "/Game/Main/Visuals/Particles/AnsaLieska.AnsaLieska" _returnvalue_3))
  (bind _asmy_game_instance (Utilities|Casting|CastToMyGameInstance (Game|GetGameInstance)))
  (Audio|PlaySoundatLocation "/Game/Main/Audio/Enviroment/Lieska.Lieska" _returnvalue_3 (* (Variables|/Game/Main/Blueprints/MyGameInstance.MyGameInstance_C|GetMasterVolume _asmy_game_instance) 1.0) 0.95 0.0 "/Game/Main/Audio/Ansa_Attenuation.Ansa_Attenuation")
  (Utilities|FlowControl|Delay 2.5)
  (Variables|Default|SetLuukkuAuki false)
  (Components|DestroyComponent _returnvalue_4)
  (Utilities|FlowControl|Delay (Math|Random|RandomFloatinRange 1.0 5.0))
  (goto _label))

(event Collision|EventActorEndOverlap
  (params (OtherActor :type Actor%20Object%20Reference))
  (bind _asbot_character (Utilities|Casting|CastTobotCharacter OtherActor))
  (Utilities|FlowControl|Delay 0.25)
  (Variables|/Game/Main/Blueprints/Pawn/botCharacter.botCharacter_C|SetDeathBy _asbot_character "NewEnumerator5"))

(event EventTick
  (params (DeltaSeconds :type Float%20%28single-precision%29))
  (if (Variables|Default|GetLuukkuAuki)
    (for _array_element (Collision|GetOverlappingActors (Variables|Default|GetBox) "/Script/Engine.Pawn" :!class /Script/Engine.PrimitiveComponent)
      (bind _asfirst_person_character (Utilities|Casting|CastToFirstPersonCharacter _array_element)
        (:then
          (Default|FeuerFrei _asfirst_person_character 0.1))
        (:CastFailed
          (bind _asbot_character (Utilities|Casting|CastTobotCharacter _array_element))
          (Default|FeuerFrei _asbot_character 0.2 "NewEnumerator4"))))))

(fn ConstructionScript)